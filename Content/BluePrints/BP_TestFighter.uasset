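; Test fighter character with forward movement, jump, and prototype ranged, melee and rotating attacks against BP_TestDummy.
; Ranged and melee inputs run debug-drawn sphere traces of different reach and damage a hit dummy, scaling only the forward vector's X component.
; The M key repositions the sphere controller and collision, then a timeline eases the collision's relative rotation through a swing.
; The rotating attack applies no damage here.
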(event EventBeginPlay
  ;[1 1 1] Rotating attack
  (Variables|Default|SetInit%20AttackController%20Location "0,75.000000, 0")
  (Variables|Default|SetInit%20AttackCollision%20Location "0,75.000000, 0")
  (Variables|Default|SetInit%20AttackRotation "60.000000, 0, 0")
  (Variables|Default|SetEnd%20AttackRotation "0, 0, 0"))

(event Input|ActionEvents|InputActionActM_jump
  (params (Key :type Key%20Structure))
  ;[1 1 1] Basic Movement
  (:Pressed
    (Character|Jump)))

(event Input|ActionEvents|InputActionActM_MeleeAttack
  (params (Key :type Key%20Structure))
  (bind _returnvalue (Transformation|GetActorLocation))
  (bind _returnvalue_2 (Transformation|GetActorForwardVector))
  ;[1 1 1] Melee Attack
  (:Pressed
    (bind _outhit (Collision|SphereTraceForObjects _returnvalue (+ _returnvalue (Math|Vector|MakeVector (* (.x _returnvalue_2) 75.0) (.y _returnvalue_2) (.z _returnvalue_2))) 5e+01 (Utilities|Array|MakeArray "ObjectTypeQuery2") false 0 "ForDuration" true "(R=1.000000,G=0.000000,B=0.000000,A=1.000000)" "(R=0.000000,G=1.000000,B=0.000000,A=1.000000)" 1.0))
    (bind _asbp_test_dummy (Utilities|Casting|CastToBP_TestDummy (.hitactor _outhit)))
    (Default|TakeDamage _asbp_test_dummy 4e+02)))

(event Input|ActionEvents|InputActionActM_RangedAttack
  (params (Key :type Key%20Structure))
  (bind _returnvalue (Transformation|GetActorLocation))
  (bind _returnvalue_2 (Transformation|GetActorForwardVector))
  ;[1 1 1] Ranged Attack
  (:Pressed
    (bind _outhit (Collision|SphereTraceForObjects _returnvalue (+ _returnvalue (Math|Vector|MakeVector (* (.x _returnvalue_2) 5e+02) (.y _returnvalue_2) (.z _returnvalue_2))) 5e+01 (Utilities|Array|MakeArray "ObjectTypeQuery2") false 0 "ForDuration" true "(R=1.000000,G=0.000000,B=0.000000,A=1.000000)" "(R=0.000000,G=1.000000,B=0.000000,A=1.000000)" 1.0))
    (bind _asbp_test_dummy (Utilities|Casting|CastToBP_TestDummy (.hitactor _outhit)))
    (Default|TakeDamage _asbp_test_dummy 1e+02)))

(event Input|AxisEvents|InputAxisAxisM_MoveLAt
  (params (AxisValue :type Float%20%28single-precision%29))
  ;[1 1 1] Basic Movement
  (Pawn|Input|AddMovementInput (Transformation|GetActorForwardVector) AxisValue false))

(event Input|KeyboardEvents|M
  (params (Key :type Key%20Structure))
  ;[1 1 1] Rotating attack
  (:Pressed
    (Transformation|SetRelativeLocation (Variables|Default|GetSphere%20Controller) (Variables|Default|GetInit%20AttackController%20Location) false false)
    (Transformation|SetRelativeLocation (Variables|Default|GetShpere%20Collision) (Variables|Default|GetInit%20AttackCollision%20Location) false false)
    (if (not (Audio|Components|Audio|IsPlaying (Variables|Default|GetTimeL_Attack03)))
      (bind _value_0___1_over_0_5s (Timeline|TimeL_Attack03 PlayFromStart)
        (:Update
          (Transformation|SetRelativeRotation (Variables|Default|GetShpere%20Collision) (Math|Interpolation|Ease "Linear" _value_0___1_over_0_5s (Variables|Default|GetInit%20AttackRotation) (Variables|Default|GetEnd%20AttackRotation) true) false false))))))

(fn ConstructionScript)