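; Test player character for a side-scrolling game with running, jumping and three attacks.
; Input is cached into variables, and Tick runs an enum state machine whose per-state graphs handle movement and transitions, with optional on-screen debug printing.
; Attack timelines animate a pivoted overlap volume, with medium and heavy attacks also launching the character.
; Flipbook switching and dialogue exit are disconnected, and Turning, Apex and Stunned have no exit transitions.
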(event Custom|Event_StateUpdater
  ;[1 1 1] Character State Machine
  (switch Utilities|FlowControl|Switch|SwitchonEnum_CharacterStates (Variables|Default|GetVar_CharStateRef)
    (:NewEnumerator0
      (CallFunction|EventStanding))
    (:NewEnumerator1
      (CallFunction|EventRunning))
    (:NewEnumerator7
      (CallFunction|EventTurning))
    (:NewEnumerator2
      (CallFunction|EventRising))
    (:NewEnumerator6
      (CallFunction|EventApex))
    (:NewEnumerator3
      (CallFunction|EventFalling))
    (:NewEnumerator4
      (CallFunction|EventAttacking))
    (:NewEnumerator5
      (CallFunction|EventStunned))))

(event Custom|Event_Standing
  ;[1 1 1] Character State Machine
  (CallFunction|EventFBUpdater)
  (|CG_Standing))

(event Custom|Event_Turning
  ;[1 1 1] Character State Machine
  (CallFunction|EventFBUpdater)
  (Utilities|FlowControl|Sequence
    (:then_0
      (CallFunction|FunAddMoveInput))))

(event Custom|Event_FBUpdater)

(event Custom|Event_Running
  ;[1 1 1] Character State Machine
  (CallFunction|EventFBUpdater)
  (|CG_Running))

(event Custom|Event_Rising
  ;[1 1 1] Character State Machine
  (CallFunction|EventFBUpdater)
  (|CG_Rising))

(event Custom|Event_Falling
  ;[1 1 1] Character State Machine
  (CallFunction|EventFBUpdater)
  (|CG_Falling))

(event Custom|Event_Attacking
  ;[1 1 1] Character State Machine
  (CallFunction|EventFBUpdater)
  (|CG_Attacking))

(event Custom|Event_Stunned
  ;[1 1 1] Character State Machine
  (CallFunction|EventFBUpdater))

(event Custom|Event_PrintDebug
  ;[1 1 1] Debug Information
  (Development|PrintString (Utilities|String|Append "Hvy Atk Input: " (Utilities|String|ToString(Boolean) (Variables|Default|GetVar_FaceRight))) true true "(R=0.000000,G=0.660000,B=1.000000,A=1.000000)" (Variables|Default|GetVar_DebugPrintTime))
  (Development|PrintString (Utilities|String|Append "Med Atk Input: " (Utilities|String|ToString(Boolean) (Variables|Default|GetVar_FaceTop))) true true "(R=0.000000,G=0.660000,B=1.000000,A=1.000000)" (Variables|Default|GetVar_DebugPrintTime))
  (Development|PrintString (Utilities|String|Append "Lght Atk Input: " (Utilities|String|ToString(Boolean) (Variables|Default|GetVar_FaceLeft))) true true "(R=0.000000,G=0.660000,B=1.000000,A=1.000000)" (Variables|Default|GetVar_DebugPrintTime))
  (Development|PrintString (Utilities|String|Append "Jump Input: " (Utilities|String|ToString(Boolean) (Variables|Default|GetVar_FaceBot))) true true "(R=0.000000,G=0.660000,B=1.000000,A=1.000000)" (Variables|Default|GetVar_DebugPrintTime))
  (Development|PrintString (Utilities|String|Append "Prime Y Axis: " (Utilities|String|ToString(Float) (Variables|Default|GetVar_VertPrime))) true true "(R=0.000000,G=0.660000,B=1.000000,A=1.000000)" (Variables|Default|GetVar_DebugPrintTime))
  (Development|PrintString (Utilities|String|Append "Prime X Axis: " (Utilities|String|ToString(Float) (Variables|Default|GetVar_LatPrime))) true true "(R=0.000000,G=0.660000,B=1.000000,A=1.000000)" (Variables|Default|GetVar_DebugPrintTime))
  (Development|PrintString (Utilities|String|Append "State: " (Utilities|String|EnumtoString (Variables|Default|GetVar_CharStateRef))) true true "(R=0.000000,G=0.660000,B=1.000000,A=1.000000)" (Variables|Default|GetVar_DebugPrintTime)))

(event Custom|Event_InDiolog
  (if (Variables|Default|GetVar_FaceRight)
    (bind _asnpc (Utilities|Casting|CastToNPC (Variables|Default|GetNPC_Refernce)))
    (Default|EndDiolog _asnpc)
    (bind _asnpcontroller (Utilities|Casting|CastToNPController (Variables|Default|GetNPC_Controller)))
    (Widget|RemovefromParent _asnpcontroller)))

(event Custom|Event_Apex
  ;[1 1 1] Character State Machine
  (CallFunction|EventFBUpdater))

(event EventBeginPlay
  ;[1 1 1] Inits and Ticks
  (Variables|/Script/Engine.PrimitiveComponent|SetbGenerateOverlapEvents (Variables|Default|GetCom_AttackVolume) false))

(event EventTick
  (params (DeltaSeconds :type Float%20%28single-precision%29))
  ;[1 1 1] Inits and Ticks
  (Variables|Default|SetVar_DebugPrintTime DeltaSeconds)
  (Utilities|FlowControl|Sequence
    (:then_0
      (if (Variables|Default|GetVar_TurnOnDebug)
        (CallFunction|EventPrintDebug)))
    (:then_1
      (CallFunction|EventStateUpdater))))

(event Input|ActionEvents|InputActionActM_FaceBottom
  (params (Key :type Key%20Structure))
  ;[1 1 1] Sets all input to local variables
  (:Pressed
    (Variables|Default|SetVar_FaceBot true))
  (:Released
    (Variables|Default|SetVar_FaceBot false)))

(event Input|ActionEvents|InputActionActM_FaceLeft
  (params (Key :type Key%20Structure))
  ;[1 1 1] Sets all input to local variables
  (:Pressed
    (Variables|Default|SetVar_FaceLeft true))
  (:Released
    (Variables|Default|SetVar_FaceLeft false)))

(event Input|ActionEvents|InputActionActM_FaceTop
  (params (Key :type Key%20Structure))
  ;[1 1 1] Sets all input to local variables
  (:Pressed
    (Variables|Default|SetVar_FaceTop true))
  (:Released
    (Variables|Default|SetVar_FaceTop false)))

(event Input|ActionEvents|InputActionActM_FaceRight
  (params (Key :type Key%20Structure))
  ;[1 1 1] Sets all input to local variables
  (:Pressed
    (Variables|Default|SetVar_FaceRight true))
  (:Released
    (Variables|Default|SetVar_FaceRight false)))

(event Input|AxisEvents|InputAxisAxisM_LateralPrime
  (params (AxisValue :type Float%20%28single-precision%29))
  ;[1 1 1] Sets all input to local variables
  (Variables|Default|SetVar_LatPrime AxisValue))

(event Input|AxisEvents|InputAxisAxisM_VerticalPrime
  (params (AxisValue :type Float%20%28single-precision%29))
  ;[1 1 1] Sets all input to local variables
  (Variables|Default|SetVar_VertPrime AxisValue))

(fn ConstructionScript)

(fn FunAddMoveInput
  (Pawn|Input|AddMovementInput "1.000000, 0, 0" (Variables|Default|GetVar_LatPrime) false)
  (Math|Float|CompareFloat (Variables|Default|GetVar_LatPrime) 0.0
    (:>
      (Pawn|SetControlRotation (Pawn|GetController) (Math|Rotator|MakeRotator 0.0 0.0 0.0)))
    (:<
      (Pawn|SetControlRotation (Pawn|GetController) (Math|Rotator|MakeRotator 0.0 0.0 1.8e+02)))))