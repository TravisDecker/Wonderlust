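; Paper2D skeleton enemy that walks horizontally toward player 0's character.
; Each Tick, while SpawnAnimation is false, it compares X positions, adds movement input scaled by CharacterMoveScale and sets yaw to face its travel direction.
; A rise-from-ground flipbook sequence, with a timeline that clears SpawnAnimation and switches to the regular skeleton flipbook, is present but disconnected and never runs.
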(event OnComponentHit(PaperFlipbook)
  (params (HitComponent :type Primitive%20Component%20Object%20Reference) (OtherActor :type Actor%20Object%20Reference) (OtherComp :type Primitive%20Component%20Object%20Reference) (NormalImpulse :type Vector :default "0, 0, 0") (Hit :type Hit%20Result%20Structure%20%28by%20ref%29)))

(event EventTick
  (params (DeltaSeconds :type Float%20%28single-precision%29))
  (bind _character_move_scale (Variables|Default|GetCharacter%20Move%20Scale))
  (if (not (Variables|Default|GetSpawn%20Animation))
    (Math|Float|CompareFloat (.x (Transformation|GetActorLocation (Game|GetPlayerCharacter 0))) (.x (Transformation|GetActorLocation))
      (:>
        (Pawn|Input|AddMovementInput "1.000000,0.0,0.0" _character_move_scale false)
        (Transformation|SetActorRotation (Math|Rotator|MakeRotator 0.0 0.0 1.8e+02)))
      (:<
        (Pawn|Input|AddMovementInput "-1.000000, 0, 0" _character_move_scale false)
        (Transformation|SetActorRotation (Math|Rotator|MakeRotator 0.0 0.0 0.0))))))

(fn ConstructionScript)