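; Mode_WonderLust, apparently a game mode, builds a chain of forest segments eastward when play begins.
; BeginPlay calls Fun_AddEastSegment in a short fixed loop, spawning each BP_ForestSegment at the stored connection point transform.
; Each new segment finds its east connection, which becomes the next spawn transform after a fixed offset along world X.
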(event EventBeginPlay
  (for _index (range 0 1)
    (CallFunction|FunAddEastSegment)))

(fn ConstructionScript)

(fn FunAddEastSegment
  (bind _returnvalue (Game|SpawnActorfromClass "/Game/BluePrints/BP_ForestSegment.BP_ForestSegment_C" (Variables|Default|GetVar_ConnectionPoint) "Undefined" 0 0))
  (bind _asbp_forest_segment (Utilities|Casting|CastToBP_ForestSegment _returnvalue))
  (Default|EventFindEastConnection _asbp_forest_segment)
  (Variables|Default|SetVar_ConnectionPoint (Math|Transform|MakeTransform (Math|Vector|MakeVector (+ (.X (Math|Vector|BreakVector (.Location (Math|Transform|BreakTransform (Variables|/Game/BluePrints/BP_ForestSegment.BP_ForestSegment_C|GetVar_EastConnection _asbp_forest_segment))))) 5e+02) (.Y (Math|Vector|BreakVector (.Location (Math|Transform|BreakTransform (Variables|/Game/BluePrints/BP_ForestSegment.BP_ForestSegment_C|GetVar_EastConnection _asbp_forest_segment))))) (.Z (Math|Vector|BreakVector (.Location (Math|Transform|BreakTransform (Variables|/Game/BluePrints/BP_ForestSegment.BP_ForestSegment_C|GetVar_EastConnection _asbp_forest_segment)))))) (.Rotation (Math|Transform|BreakTransform (Variables|/Game/BluePrints/BP_ForestSegment.BP_ForestSegment_C|GetVar_EastConnection _asbp_forest_segment))) (.Scale (Math|Transform|BreakTransform (Variables|/Game/BluePrints/BP_ForestSegment.BP_ForestSegment_C|GetVar_EastConnection _asbp_forest_segment))))))