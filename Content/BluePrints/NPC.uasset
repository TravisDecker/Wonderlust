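; NPC actor that shows dialogue and can follow the player along the X axis.
; Collision overlap displays the current dialogue line in a TextRender, creates an NPController widget and passes itself and the widget to BP_AlphaPlayer.
; Ending overlap removes the widget, while EndDiolog hides the text.
; Once followplayer sets IsFollowing, Tick snaps the NPC 100 units behind the player whenever the player's X is greater.
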(event OnComponentBeginOverlap(CollisionBox)
  (params (OverlappedComponent :type Primitive%20Component%20Object%20Reference) (OtherActor :type Actor%20Object%20Reference) (OtherComp :type Primitive%20Component%20Object%20Reference) (OtherBodyIndex :type Integer) (bFromSweep :type Boolean) (SweepResult :type Hit%20Result%20Structure%20%28by%20ref%29))
  ;[1 1 1] Diolog controle
  (bind _asbp_alpha_player (Utilities|Casting|CastToBP_AlphaPlayer (Game|GetPlayerCharacter 0)))
  (Variables|/Game/BP_AlphaPlayer.BP_AlphaPlayer_C|SetNPC_Refernce _asbp_alpha_player self)
  (Rendering|Components|TextRender|SetText (Variables|Default|GetTextRender) (Utilities|Array|Get(acopy) (Variables|Default|GetNPCDiolog) (Variables|Default|GetDiologIndex)))
  (Rendering|SetVisibility (Variables|Default|GetTextRender) true false)
  (bind _returnvalue (UserInterface|CreateWidget "/Game/BluePrints/UMG/NPController.NPController_C"))
  (UserInterface|Viewport|AddtoViewport _returnvalue 0)
  (Variables|Default|SetNPC_Controller _returnvalue)
  (bind _asbp_alpha_player_2 (Utilities|Casting|CastToBP_AlphaPlayer (Game|GetPlayerCharacter 0)))
  (Variables|/Game/BP_AlphaPlayer.BP_AlphaPlayer_C|SetNPC_Controller _asbp_alpha_player_2 _returnvalue))

(event OnComponentEndOverlap(CollisionBox)
  (params (OverlappedComponent :type Primitive%20Component%20Object%20Reference) (OtherActor :type Actor%20Object%20Reference) (OtherComp :type Primitive%20Component%20Object%20Reference) (OtherBodyIndex :type Integer))
  ;[1 1 1] Diolog controle
  (bind _asnpcontroller (Utilities|Casting|CastToNPController (Variables|Default|GetNPC_Controller)))
  (Widget|RemovefromParent _asnpcontroller))

(event Custom|End%20Diolog
  ;[1 1 1] Diolog controle
  (Rendering|SetVisibility (Variables|Default|GetTextRender) false false))

(event Custom|follow%20player
  (bind _output_get (Variables|Default|SetIsFollowing true)))

(event EventTick
  (params (DeltaSeconds :type Float%20%28single-precision%29))
  (bind _returnvalue (Transformation|GetActorLocation))
  (if (stale Custom|follow%20player _output_get)
    (Variables|Default|SetPlayer%20Location (.x (Transformation|GetActorLocation (Game|GetPlayerCharacter 0))))
    (Variables|Default|SetNPC%20follow%20location (.x _returnvalue))
    (if (> (Variables|Default|GetPlayer%20Location) (Variables|Default|GetNPC%20follow%20location))
      (Development|PrintString "Follow" true true "(R=0.904624,G=1.000000,B=0.199084,A=1.000000)")
      (Transformation|SetActorLocation (Math|Vector|MakeVector (- (Variables|Default|GetPlayer%20Location) 1e+02) (.y _returnvalue) (.z _returnvalue)) false false))))

(fn ConstructionScript)