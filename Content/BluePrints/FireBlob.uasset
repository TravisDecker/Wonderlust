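; FireBlob is a pawn that applies movement input every Tick, apparently intended to chase player 0.
; The input vector is its own world location plus a small, frame-time-scaled step toward the player, so it is not a pure direction to the player.
; An X-axis comparison move and a SetActorLocation call are left unconnected, and Possessed and the construction script are empty.
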(event EventTick
  (params (DeltaSeconds :type Float%20%28single-precision%29))
  (bind _returnvalue (Transformation|GetActorLocation))
  (Pawn|Input|AddMovementInput (+ _returnvalue (* (* (Math|Vector|Normalize (- (Transformation|GetActorLocation (Game|GetPlayerCharacter 0)) _returnvalue)) DeltaSeconds) 2e+01)) 1.0 false))

(event EventPossessed
  (params (NewController :type Controller%20Object%20Reference)))

(fn ConstructionScript)