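; BP_ForestSegment is a forest level segment that requests the next segment to the east and kills players that leave its bounds.
; On BeginPlay it caches the world transform of its east origin component as the east connection point.
; A player entering the east proximity volume makes the Mode_WonderLust game mode add an east segment.
; Upper and lower kill volumes destroy any BP_TestPlayer that overlaps them.
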(event OnComponentBeginOverlap(Com_UpperKillVol)
  (params (OverlappedComponent :type Primitive%20Component%20Object%20Reference) (OtherActor :type Actor%20Object%20Reference) (OtherComp :type Primitive%20Component%20Object%20Reference) (OtherBodyIndex :type Integer) (bFromSweep :type Boolean) (SweepResult :type Hit%20Result%20Structure%20%28by%20ref%29))
  (bind _asbp_test_player (Utilities|Casting|CastToBP_TestPlayer OtherActor))
  (Actor|DestroyActor _asbp_test_player))

(event OnComponentBeginOverlap(Com_LowerKillVol)
  (params (OverlappedComponent :type Primitive%20Component%20Object%20Reference) (OtherActor :type Actor%20Object%20Reference) (OtherComp :type Primitive%20Component%20Object%20Reference) (OtherBodyIndex :type Integer) (bFromSweep :type Boolean) (SweepResult :type Hit%20Result%20Structure%20%28by%20ref%29))
  (bind _asbp_test_player (Utilities|Casting|CastToBP_TestPlayer OtherActor))
  (Actor|DestroyActor _asbp_test_player))

(event OnComponentBeginOverlap(Com_NearActorsEast)
  (params (OverlappedComponent :type Primitive%20Component%20Object%20Reference) (OtherActor :type Actor%20Object%20Reference) (OtherComp :type Primitive%20Component%20Object%20Reference) (OtherBodyIndex :type Integer) (bFromSweep :type Boolean) (SweepResult :type Hit%20Result%20Structure%20%28by%20ref%29))
  (Utilities|Casting|CastToBP_TestPlayer OtherActor)
  (bind _asmode_wonder_lust (Utilities|Casting|CastToMode_WonderLust (Game|GetGameMode)))
  (Default|FunAddEastSegment _asmode_wonder_lust))

(event Custom|Event_FindEastConnection
  (Variables|Default|SetVar_EastConnection (Transformation|GetWorldTransform (Variables|Default|GetCom_EastOrigin))))

(event EventBeginPlay
  (CallFunction|EventFindEastConnection))

(fn ConstructionScript)