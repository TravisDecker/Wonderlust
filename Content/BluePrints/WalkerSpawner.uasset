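; Walker spawner that creates a small random batch of Walker AI at its own location once its trigger box is overlapped.
; BeginPlay rolls the batch limit, and any overlap sets a triggered flag, as the player cast never runs.
; Tick then spawns until the counter passes that limit, firing the first spawn immediately and using a short Delay to space out the rest.
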(event OnComponentBeginOverlap(Box)
  (params (OverlappedComponent :type Primitive%20Component%20Object%20Reference) (OtherActor :type Actor%20Object%20Reference) (OtherComp :type Primitive%20Component%20Object%20Reference) (OtherBodyIndex :type Integer) (bFromSweep :type Boolean) (SweepResult :type Hit%20Result%20Structure%20%28by%20ref%29))
  (Variables|Default|SetVar_Triggerd true))

(event EventBeginPlay
  (Variables|Default|SetVar_Rand (+ (Math|Random|RandomInteger 2) 1)))

(event EventTick
  (params (DeltaSeconds :type Float%20%28single-precision%29))
  (if (Variables|Default|GetVar_Triggerd)
    (if (<= (Variables|Default|GetVar_Count) (Variables|Default|GetVar_Rand))
      (if (Variables|Default|GetVar_FirstSpawn)
        (Utilities|FlowControl|Delay 0.75)
        (else
          (Variables|Default|SetVar_FirstSpawn true)))
      (AI|SpawnAIFromClass "/Game/Blueprints/Walker.Walker_C" 0 (Transformation|GetActorLocation) "0, 0, 0" false)
      (Variables|Default|SetVar_Count (+ (Variables|Default|GetVar_Count) 1)))))

(fn ConstructionScript)