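; Player character for a 2D side-scrolling game, driven by an enum state machine with flipbook animation.
; Input events cache axes and face buttons into variables, which Tick's state updater reads through per-state collapsed graphs for movement, jumping and transitions.
; Attacking sweeps a pivot by timeline, then returns to Standing.
; Stunned is empty, the dialog-exit event is never called, and a toggle prints input and state each frame.
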(event Custom|Event_StateUpdater
  ;[1 1 1] Character State Machine
  (switch Utilities|FlowControl|Switch|SwitchonEnum_CharacterStates (Variables|Default|GetVar_CharStateRef)
    (:NewEnumerator0
      (CallFunction|EventStanding))
    (:NewEnumerator1
      (CallFunction|EventRunning))
    (:NewEnumerator2
      (CallFunction|EventRising))
    (:NewEnumerator3
      (CallFunction|EventFalling))
    (:NewEnumerator4
      (CallFunction|EventAttacking))
    (:NewEnumerator5
      (CallFunction|EventStunned))))

(event Custom|Event_Standing
  ;[1 1 1] Character State Machine
  (|CG_Standing))

(event Custom|Event_Running
  ;[1 1 1] Character State Machine
  (|CG_Running))

(event Custom|Event_Rising
  ;[1 1 1] Character State Machine
  (|CG_Rising))

(event Custom|Event_Falling
  ;[1 1 1] Character State Machine
  (|CG_Falling))

(event Custom|Event_Attacking
  (Utilities|FlowControl|Sequence
    (:then_0
      (Pawn|Input|AddMovementInput "1.000000, 0, 0" (Variables|Default|GetVar_LatPrime) false)
      (Math|Float|CompareFloat (Variables|Default|GetVar_LatPrime) 0.0
        (:>
          (Pawn|SetControlRotation (Pawn|GetController) (Math|Rotator|MakeRotator 0.0 0.0 0.0)))
        (:<
          (Pawn|SetControlRotation (Pawn|GetController) (Math|Rotator|MakeRotator 0.0 0.0 1.8e+02)))))
    (:then_1
      (if (not (Audio|Components|Audio|IsPlaying (Variables|Default|GetTimeline_0)))
        (bind _newtrack_0 (Timeline|Timeline_0 PlayFromStart)
          (:Update
            (Transformation|SetRelativeRotation (Variables|Default|GetCom_AttackPivot) (Math|Interpolation|Ease "Linear" _newtrack_0 (Math|Rotator|MakeRotator 0.0 0.0 45.0) (Math|Rotator|MakeRotator 0.0 0.0 -45.0) true) false false))
          (:Finished
            (Variables|Default|SetVar_CharStateRef "NewEnumerator0")))))))

(event Custom|Event_Stunned
  ;[1 1 1] Character State Machine
)

(event Custom|Event_PrintDebug
  (Utilities|FlowControl|Sequence
    (:then_0
      (Development|PrintString (Utilities|String|ToString(Float) (Variables|Default|GetVar_LatPrime)) true true "(R=0.000000,G=0.660000,B=1.000000,A=1.000000)" (Variables|Default|GetVar_DebugPrintTime)))
    (:then_1
      (Development|PrintString (Utilities|String|ToString(Float) (Variables|Default|GetVar_VertPrime)) true true "(R=0.000000,G=0.660000,B=1.000000,A=1.000000)" (Variables|Default|GetVar_DebugPrintTime)))
    (:then_2
      (Development|PrintString (Utilities|String|ToString(Boolean) (Variables|Default|GetVar_FaceBot)) true true "(R=0.000000,G=0.660000,B=1.000000,A=1.000000)" (Variables|Default|GetVar_DebugPrintTime)))
    (:then_3
      (Development|PrintString (Utilities|String|ToString(Boolean) (Variables|Default|GetVar_FaceLeft)) true true "(R=0.000000,G=0.660000,B=1.000000,A=1.000000)" (Variables|Default|GetVar_DebugPrintTime)))
    (:then_4
      (Development|PrintString (Utilities|String|ToString(Boolean) (Variables|Default|GetVar_FaceTop)) true true "(R=0.000000,G=0.660000,B=1.000000,A=1.000000)" (Variables|Default|GetVar_DebugPrintTime)))
    (:then_5
      (Development|PrintString (Utilities|String|ToString(Boolean) (Variables|Default|GetVar_FaceRight)) true true "(R=0.000000,G=0.660000,B=1.000000,A=1.000000)" (Variables|Default|GetVar_DebugPrintTime)))
    (:then_6
      (Development|PrintString (Utilities|String|EnumtoString (Variables|Default|GetVar_CharStateRef)) true true "(R=0.000000,G=0.660000,B=1.000000,A=1.000000)" (Variables|Default|GetVar_DebugPrintTime)))))

(event Custom|Event_InDiolog
  (if (Variables|Default|GetVar_FaceRight)
    (bind _asnpc (Utilities|Casting|CastToNPC (Variables|Default|GetNPC_Refernce)))
    (Default|EndDiolog _asnpc)
    (bind _asnpcontroller (Utilities|Casting|CastToNPController (Variables|Default|GetNPC_Controller)))
    (Widget|RemovefromParent _asnpcontroller)))

(event EventTick
  (params (DeltaSeconds :type Float%20%28single-precision%29))
  (Variables|Default|SetVar_DebugPrintTime DeltaSeconds)
  (Utilities|FlowControl|Sequence
    (:then_0
      (if (Variables|Default|GetVar_TurnOnDebug)
        (CallFunction|EventPrintDebug)))
    (:then_1
      (CallFunction|EventStateUpdater))))

(event Input|ActionEvents|InputActionActM_FaceBottom
  (params (Key :type Key%20Structure))
  ;[1 1 1] Sets all input to local variables
  (:Pressed
    (Variables|Default|SetVar_FaceBot true))
  (:Released
    (Variables|Default|SetVar_FaceBot false)))

(event Input|ActionEvents|InputActionActM_FaceLeft
  (params (Key :type Key%20Structure))
  ;[1 1 1] Sets all input to local variables
  (:Pressed
    (Variables|Default|SetVar_FaceLeft true))
  (:Released
    (Variables|Default|SetVar_FaceLeft false)))

(event Input|ActionEvents|InputActionActM_FaceTop
  (params (Key :type Key%20Structure))
  ;[1 1 1] Sets all input to local variables
  (:Pressed
    (Variables|Default|SetVar_FaceTop true))
  (:Released
    (Variables|Default|SetVar_FaceTop false)))

(event Input|ActionEvents|InputActionActM_FaceRight
  (params (Key :type Key%20Structure))
  ;[1 1 1] Sets all input to local variables
  (:Pressed
    (Variables|Default|SetVar_FaceRight true))
  (:Released
    (Variables|Default|SetVar_FaceRight false)))

(event Input|AxisEvents|InputAxisAxisM_LateralPrime
  (params (AxisValue :type Float%20%28single-precision%29))
  ;[1 1 1] Sets all input to local variables
  (Variables|Default|SetVar_LatPrime AxisValue))

(event Input|AxisEvents|InputAxisAxisM_VerticalPrime
  (params (AxisValue :type Float%20%28single-precision%29))
  ;[1 1 1] Sets all input to local variables
  (Variables|Default|SetVar_VertPrime AxisValue))

(fn ConstructionScript)